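; Openable door actor that swings open and closed in response to OpenDoor interface events.
; It stores its starting rotation on BeginPlay, and the DoorSwing timeline adds a yaw offset to it each update.
; Opening plays the timeline and closing reverses it, while an event track on the timeline plays the door sound at the actor's location.
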(event `self.ReceiveBeginPlay`
  (set `self.InitialRotation` (`self.K2_GetActorRotation`)))

(event `self.OpenDoor.OnOpen`
  (bind (_direction _open_door) (`Timeline|DoorSwing` :!label _label)
    (:`Update`
      (`self.K2_SetActorRotation` (`KismetMathLibrary.ComposeRotators` (`KismetMathLibrary.MakeRotator` 0.0 0.0 _open_door) (`self.InitialRotation`))))
    (:`DoorSound`
      (`GameplayStatics.PlaySoundAtLocation` "/Game/Audio/sounDoor.sounDoor" (`self.K2_GetActorLocation`)))))

(event `self.OpenDoor.OnClose`
  (goto _label :!via `Reverse`))

(fn `UserConstructionScript`)